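; MasterNPC is an NPC Blueprint that changes to a random facial expression when the main character overlaps its Box component.
; The overlap event calls RandomExpression, which filters for MainChar_BP and casts the skeletal mesh's anim instance to NPC_ABP.
; It converts a random integer to an E_PartyFacialExpression value and passes it to the anim Blueprint through NewFacialExpressionMessage, with debug prints along the way.
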(event `self.Box.OnComponentBeginOverlap`
  (params (OverlappedComponent :type "PrimitiveComponent Object Reference") (OtherActor :type "Actor Object Reference") (OtherComp :type "PrimitiveComponent Object Reference") (OtherBodyIndex :type Integer) (bFromSweep :type Boolean) (SweepResult :type "HitResult Structure (by ref)"))
  (`self.RandomExpression` OtherActor))

(fn `RandomExpression`
  (params (NewParam :type "Actor Object Reference"))
  (cast `/Game/Blueprints/Character/MainChar_BP` NewParam
    (:`then`
      (bind _asnpc_abp (cast `/Game/Blueprints/AnimBP/NPC_ABP` (`SkeletalMeshComponent.GetAnimInstance` (`self.SkeletalMesh`))))
      (`KismetSystemLibrary.PrintString` "Bob is overlaappibng")
      (message `/Game/Blueprints/FacialExpression/BPI_FacialExpression.NewFacialExpression` _asnpc_abp (cast `/Game/Blueprints/FacialExpression/E_PartyFacialExpression` (`KismetMathLibrary.Conv_IntToByte` (`KismetMathLibrary.RandomInteger` 7)))))
    (:`CastFailed`
      (`KismetSystemLibrary.PrintString` "Bob is not read"))))

(fn `UserConstructionScript`)