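; Lobby player controller that shows the lobby HUD and manages the character displayed for selection.
; On BeginPlay it opens Lobby2HUD in UI-only input with the cursor shown, then spawns a default character at the actor tagged "Placement".
; SetCharacter destroys the current character and spawns a replacement there, taking its class from a level actor tagged with the given name.
; Leaving the level removes all widgets.
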(event `self.ReceiveBeginPlay`
  ;[1 1 1] Add Lobby HUD/UI
  (bind _returnvalue (`|CreateWidget` "/Game/Blueprints/HUD/Lobby2HUD.Lobby2HUD_C" self))
  (`UserWidget.AddToViewport` _returnvalue 0)
  (`WidgetBlueprintLibrary.SetInputMode_UIOnlyEx` self _returnvalue "LockAlways")
  (set `self.bShowMouseCursor` true)
  ;[1 1 1] Set first character in the lobby
  (bind _outactors (`GameplayStatics.GetAllActorsWithTag` "Placement"))
  (bind _output_get (set `self.PlacementLocRef` (`|GetArrayItem` _outactors)))
  (bind _returnvalue_2 (`|SpawnActorFromClass` "/Game/Blueprints/Character/BP_MR_BOB_APPROVELobby.BP_MR_BOB_APPROVELobby_C" (`KismetMathLibrary.MakeTransform` (`self.K2_GetActorLocation` _output_get) (`self.K2_GetActorRotation` _output_get)) "Undefined" "OverrideRootScale" null null))
  (set `self.Selected Actor Object Ref` _returnvalue_2))

(event `On Leaving Level`
  (`WidgetLayoutLibrary.RemoveAllWidgets`))

(fn `SetCharacter`
  (params (`LobbyChar Name` :type String))
  (bind _placementlocref (`self.PlacementLocRef`))
  (bind _selected_actor_object_ref (`self.Selected Actor Object Ref`))
  ;[1 1 1] Destroy previous character obj. ref if exist
  (`/Engine/EditorBlueprintResources/StandardMacros.IsValid` _selected_actor_object_ref
    (:`Is Valid`
      (`self.K2_DestroyActor` _selected_actor_object_ref)
      ;[1 1 1] Find available actor by tags
      (bind _outactors (`GameplayStatics.GetAllActorsOfClassWithTag` "/Script/Engine.Actor" (`KismetStringLibrary.Conv_StringToName` `LobbyChar Name`)))
      (bind _returnvalue (`|SpawnActorFromClass` (`GameplayStatics.GetObjectClass` (`|GetArrayItem` _outactors)) (`KismetMathLibrary.MakeTransform` (`self.K2_GetActorLocation` _placementlocref) (`self.K2_GetActorRotation` _placementlocref)) "Undefined" "OverrideRootScale" null null))
      ;[1 1 1] Store in variable for later destroy
      (set `self.Selected Actor Object Ref` _returnvalue))))

(fn `UserConstructionScript`)