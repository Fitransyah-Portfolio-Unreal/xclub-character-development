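; Player controller that, on BeginPlay, sets game-only input and passes the game instance's SelectedCharacter to SetCharacter, whose body is not shown here.
; An unconnected chain would possess the tag-matched MainChar_BP at the "Placement" actor and destroy the others, defaulting to "GameChar1".
; SpawnDefaultPawn, uncalled here, possesses the first available character at that placement, relying on variables only that dead chain sets.
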(event `self.ReceiveBeginPlay`
  ;[1 1 1] Initialization at begin play
  (`WidgetBlueprintLibrary.SetInputMode_GameOnly` self)
  (bind _asxclub_game_instance_bp (cast `/Game/Blueprints/GameSetting/XClub_GameInstance_BP` (`GameplayStatics.GetGameInstance`)))
  (`self.SetCharacter` (`XClub_GameInstance.SelectedCharacter` _asxclub_game_instance_bp)))

(fn `Spawn Default Pawn`
  (bind _placementlocref (`self.PlacementLocRef`))
  (bind _output (`|GetArrayItem` (`self.AvailableCharacter`)))
  (`self.K2_SetActorLocationAndRotation` _output (`self.K2_GetActorLocation` _placementlocref) (`self.K2_GetActorRotation` _placementlocref) false false)
  (`self.Possess` self _output))

(fn `UserConstructionScript`)