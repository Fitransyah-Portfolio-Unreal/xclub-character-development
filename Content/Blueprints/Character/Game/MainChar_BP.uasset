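; Main character Blueprint that handles dancing, body-fall effects and debug controls for drunkenness and face capture.
; Start and stop events toggle the dancing flag, with dancing blocked while the drunk state is Wasted.
; Fall events spawn a dust actor and play a thud sound at an offset from the mesh.
; Debug keys raise or lower drunkenness, print available Live Link subjects and enable face Live Link.
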(event `self.ReceiveBeginPlay`)

(event `self.StartDancing`
  ;[1 1 1] Dance Configuration
  (if (`|EnumInequality` (`self.DrunkState`) "EDL_Wasted")
    (set `self.bIsDancing` true)))

(event `self.StopDancing`
  ;[1 1 1] Dance Configuration
  (set `self.bIsDancing` false))

(event `DustFromBody`
  ;[1 1 1] End Fall Effect
  (`|SpawnActorFromClass` "/Game/Blueprints/PS_DustBP.PS_DustBP_C" (`KismetMathLibrary.MakeTransform` (+ (`SceneComponent.K2_GetComponentLocation` (`self.Mesh`)) (`KismetMathLibrary.MakeVector` 0.0 -80.0))) "Undefined" "OverrideRootScale" null null))

(event `FallToGroundSound`
  ;[1 1 1] End Fall Effect
  (`GameplayStatics.PlaySoundAtLocation` "/Game/Assets/Audio/Sfx/Body_fall-sound_effect-YoutubeConvert_cc_Cue.Body_fall-sound_effect-YoutubeConvert_cc_Cue" (+ (`SceneComponent.K2_GetComponentLocation` (`self.Mesh`)) (`KismetMathLibrary.MakeVector` 0.0 -80.0)) (struct) 1.0 1.0 0.0 null null null null))

(event `Key|P`
  (params (Key :type "Key Structure"))
  ;[1 1 1] Debugging
  (:`Pressed`
    (set `self.Drunkness` (+ (`self.Drunkness`) (`self.IntoxicationRate`)))))

(event `Key|O`
  (params (Key :type "Key Structure"))
  ;[1 1 1] Debugging
  (:`Pressed`
    (set `self.Drunkness` (- (`self.Drunkness`) (`self.IntoxicationRate`)))))

(event `Key|U`
  (params (Key :type "Key Structure"))
  ;[1 1 1] Debugging
  (:`Pressed`
    (bind _returnvalue (`LiveLinkBlueprintLibrary.GetLiveLinkSubjects` false))
    (if (> (`KismetArrayLibrary.Array_Length` _returnvalue) 0)
      (`KismetSystemLibrary.PrintString` "There is subject available")
      (for _array_element _returnvalue
        (`KismetSystemLibrary.PrintString` (`KismetStringLibrary.Conv_NameToString` (`.Name` (break `LiveLinkSubjectName` (`.SubjectName` (break `LiveLinkSubjectKey` _array_element)))))))
      (else
        (`KismetSystemLibrary.PrintString` "There is NO subject available")))))

(event `Key|Y`
  (params (Key :type "Key Structure"))
  ;[1 1 1] Debugging
  (:`Pressed`
    (set `self.bFaceLiveLinkEnabled` true)
    (`KismetSystemLibrary.PrintString` "Face Live Link already enabled" true true (struct :`G` 1.0 :`B` 0.159328 :`A` 1.0))))

(fn `UserConstructionScript`)